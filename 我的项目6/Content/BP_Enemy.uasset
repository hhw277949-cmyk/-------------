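; BP_Enemy is an enemy that chases the player and attacks at close range.
; Every Tick spawns and attaches a new pistol to the hand_r socket and reissues AIMoveTo toward the player.
; A DoOnce with a delayed reset throttles the attack, which plays a montage and applies damage directly after distance checks.
; AnyDamage reduces Health; death increments the game mode's score, prints victory at the target, and destroys the enemy.
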(event `self.ReceiveTick`
  (params (DeltaSeconds :type "Float (single-precision)"))
  (bind _returnvalue (`GameplayStatics.GetPlayerCharacter` 0))
  (bind _returnvalue_2 (`|SpawnActorFromClass` "/Game/Variant_Shooter/Blueprints/Pickups/Weapons/BP_ShooterWeapon_Pistol.BP_ShooterWeapon_Pistol_C" (`self.GetTransform`) "AlwaysSpawn" "MultiplyWithRoot" self null))
  (`self.K2_AttachToComponent` _returnvalue_2 (`self.Mesh`) "hand_r" "SnapToTarget" "SnapToTarget" "SnapToTarget" true)
  (`self.K2_AddActorLocalRotation` _returnvalue_2 (struct :`Pitch` 10.0 :`Yaw` 90.0 :`Roll` 10.0) false false)
  (`|AIMoveTo` self (0.0 0.0 0.0) _returnvalue 100.0
    (:`then`
      (if (<= (`self.GetDistanceTo` _returnvalue null) 120.0)
        (`/Engine/EditorBlueprintResources/StandardMacros.DoOnce` false :!label _label
          (:`Completed`
            (if (<= (`self.GetDistanceTo` (`GameplayStatics.GetPlayerCharacter` 0)) 150.0)
              (`self.PlayAnimMontage` "/Game/Characters/Mannequins/Anims/Unarmed/Attack/AM_EnemyAttack.AM_EnemyAttack")
              (`GameplayStatics.ApplyDamage` _returnvalue 10.0)
              (`KismetSystemLibrary.PrintString` "ATTACK HIT!"))
            (`KismetSystemLibrary.Delay` 1.0)
            (goto _label :!via `Reset`)))))))

(event `self.ReceiveAnyDamage`
  (params (Damage :type "Float (single-precision)") (DamageType :type "DamageType Object Reference") (InstigatedBy :type "Controller Object Reference") (DamageCauser :type "Actor Object Reference"))
  (bind _output_get (set `self.Health` (- (`self.Health`) Damage)))
  (if (<= _output_get 0.0)
    (bind _asbp_first_person_game_mode (cast `/Game/FirstPerson/Blueprints/BP_FirstPersonGameMode` (`GameplayStatics.GetGameMode`)))
    (bind _output_get_2 (set `/Game/FirstPerson/Blueprints/BP_FirstPersonGameMode.Score` (+ (`/Game/FirstPerson/Blueprints/BP_FirstPersonGameMode.Score` _asbp_first_person_game_mode) 1) _asbp_first_person_game_mode))
    (if (>= _output_get_2 (`/Game/FirstPerson/Blueprints/BP_FirstPersonGameMode.TargetScore` _asbp_first_person_game_mode))
      (`KismetSystemLibrary.PrintString` "VICTORY! YOU WIN!" true true (struct :`R` 0.991304 :`A` 1.0) 10.0))
    (`self.K2_DestroyActor`)))

(fn `UserConstructionScript`)